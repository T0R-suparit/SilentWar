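; Portal actor meant to teleport MainCharacter between paired portals, with its mesh and exit point placed by the construction script.
; On hit, it loops over all Portal_BP actors and uses the last one's Exit as destination.
; Entry portals move the character there; non-entry portals move themselves instead.
; PortalIndex and Entry/exit matching checks exist but are disconnected, so pairing never takes effect.
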(event `self.ReceiveHit`
  (params (MyComp :type "PrimitiveComponent Object Reference") (Other :type "Actor Object Reference") (OtherComp :type "PrimitiveComponent Object Reference") (bSelfMoved :type Boolean) (HitLocation :type "Vector Structure") (HitNormal :type "Vector Structure") (NormalImpulse :type "Vector Structure") (Hit :type "HitResult Structure (by ref)"))
  (bind _asmain_character (cast `/Game/Character/Main/MainCharacter` Other))
  (if (`self.Entry?`)
    (bind _outactors (`GameplayStatics.GetAllActorsOfClass` "Portal_BP_C"))
    (for _array_element _outactors
      _)
    (`self.K2_SetActorLocation` _asmain_character (`SceneComponent.K2_GetComponentLocation` (`/Game/Object/Portal/Portal_BP.Exit` _array_element)) false false)
    (else
      (bind _outactors_2 (`GameplayStatics.GetAllActorsOfClass` "Portal_BP_C"))
      (for _array_element_2 _outactors_2
        _)
      (`self.K2_SetActorLocation` (`SceneComponent.K2_GetComponentLocation` (`/Game/Object/Portal/Portal_BP.Exit` _array_element_2))))))

(fn `UserConstructionScript`
  (`SceneComponent.K2_SetRelativeTransform` (`self.Portal`) (`self.Portal Transform`) false false)
  (`SceneComponent.K2_SetRelativeLocation` (`self.Exit`) (`self.Exit Location`) false false))